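; BP_PlantSpawner is an actor that respawns a plant of a set class whenever none is found nearby.
; BeginPlay starts a looping timer at CheckFrequency, presumably driving SpawnerTick, which sphere-traces the Radius for actors of exactly PlantClass.
; If none is hit, it picks a random direction scaled by Radius, snaps that point to static-world floor and spawns one plant there.
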(event `self.ReceiveBeginPlay`
  (`KismetSystemLibrary.K2_SetTimerDelegate` (`|CreateDelegate` :!event `SpawnerTick`) (`self.CheckFrequency`) true))

(fn `SpawnerTick`
  (bind _returnvalue (`self.K2_GetActorLocation`))
  (bind _outhits (`KismetSystemLibrary.SphereTraceMultiForObjects` _returnvalue _returnvalue (`self.Radius`) (`|MakeArray` "ObjectTypeQuery2" "ObjectTypeQuery1" "ObjectTypeQuery3" "ObjectTypeQuery4" :!type "EObjectTypeQuery Enum") true))
  (for _array_element _outhits
    (if (== (`GameplayStatics.GetObjectClass` (`.HitActor` (`GameplayStatics.BreakHitResult` _array_element))) (`self.PlantClass`))
      (return)))
  (`|SpawnActorFromClass` (`self.PlantClass`) (`KismetMathLibrary.MakeTransform` (`/Game/BP/BP_FunctionLibrary.SnapToFloor` (+ (* (`KismetMathLibrary.RandomUnitVector`) (`self.Radius`)) (`self.K2_GetActorLocation`)) 2000.0 2000.0 (`|MakeArray` "ObjectTypeQuery1" :!type "EObjectTypeQuery Enum"))) "AdjustIfPossibleButAlwaysSpawn" "OverrideRootScale" null null))

(fn `UserConstructionScript`)