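; BP_PlantBase is a base actor for plants that serve as food and have a limited lifetime.
; On BeginPlay it binds one handler to both the lifetime component's end event and the food component's calories-ended event, so either destroys the plant.
; Three getter functions expose its single Cube component as the target for appearance, color and size updates.
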(event `self.ReceiveBeginPlay`
  (add `/Game/BP/Components/BP_LifetimeComponent.OnLifetimeEnded` (`self.BP_LifetimeComponent`) (delegate `OnLifetimeEnded_Event_0`))
  (add `/Game/BP/Components/BP_FoodComponent.CaloriesEnded` (`self.BP_FoodComponent`) (delegate `OnLifetimeEnded_Event_0`)))

(event `OnLifetimeEnded_Event_0`
  (`self.K2_DestroyActor`))

(fn `GetAppearanceComponents`
  (returns (Components :type "Array of SceneComponent Object Reference"))
  (return (`|MakeArray` (`self.Cube`) :!type "SceneComponent Object Reference")))

(fn `GetComponentsToUpdateColor`
  (returns (Components :type "Array of SceneComponent Object Reference"))
  (return (`|MakeArray` (`self.Cube`) :!type "SceneComponent Object Reference")))

(fn `GetComponentsToUpdateSize`
  (returns (Components :type "Array of SceneComponent Object Reference"))
  (return (`|MakeArray` (`self.Cube`) :!type "SceneComponent Object Reference")))

(fn `UserConstructionScript`)