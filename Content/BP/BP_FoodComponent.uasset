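; BP_FoodComponent is a food component that stores a calorie amount that can be consumed.
; BeginPlay fills Calories from DefaultCalories when it is zero, and the setter clamps it to a fixed range.
; ConsumeCalories deducts up to the requested amount, returns what was consumed and whether that fully satisfied the request, and fires CaloriesEnded on depletion.
; GetFoodState is an empty stub.
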(event `self.ReceiveBeginPlay`
  (if (== (`self.Calories`) 0.0)
    (set `self.Calories` (`self.DefaultCalories`))))

(fn `ConsumeCalories`
  (params (RequestedCalories :type "Float (double-precision)"))
  (returns (ConsumedCalories :type "Float (double-precision)") (IsRequestFullySatisfied :type Boolean))
  (locals (CaloriesConsumed :type "Float (double-precision)"))
  (if (<= RequestedCalories (`self.Calories`))
    (`self.SetCurrentCalories` (- (`self.Calories`) (`local.RequestedCalories`)))
    (if (`KismetMathLibrary.NearlyEqual_FloatFloat` (`self.Calories`))
      (`self.CaloriesEnded`))
    (return (`local.RequestedCalories`) true)
    (else
      (set `local.CaloriesConsumed` (`self.Calories`))
      (`self.SetCurrentCalories` 0.0)
      (`self.CaloriesEnded`)
      (return (`local.CaloriesConsumed`) false))))

(fn `GetCurrentCalories`
  (returns (Calories :type "Float (double-precision)"))
  (return (`self.Calories`)))

(fn `GetFoodState`)

(fn `SetCurrentCalories`
  (params (Calories :type "Float (double-precision)"))
  (set `self.Calories` (`KismetMathLibrary.FClamp` Calories 0.0 10000.0)))