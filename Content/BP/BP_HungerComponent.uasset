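; Hunger component that stores a Hunger value and changes it by a set amount per update.
; BeginPlay starts a looping timer at UpdateFrequency, with a start-delay variance of half that interval to stagger instances.
; UpdateHunger, the apparent timer target, adds UpdateAmount through the GetHunger and SetHunger accessors, with no clamping.
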(event `self.ReceiveBeginPlay`
  (bind _updatefrequency (`self.UpdateFrequency`))
  (`KismetSystemLibrary.K2_SetTimerDelegate` (`|CreateDelegate` :!event `UpdateHunger`) _updatefrequency true 0.0 (/ _updatefrequency 2.0)))

(fn `GetHunger`
  (returns (Hunger :type "Float (double-precision)"))
  (return (`self.Hunger`)))

(fn `SetHunger`
  (params (Hunger :type "Float (double-precision)"))
  (set `self.Hunger` Hunger))

(fn `UpdateHunger`
  (`self.SetHunger` (+ (`self.GetHunger`) (`self.UpdateAmount`))))