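; Player controller for an animal simulation, handling pause and settings menus, HUD modes, saved sensitivity and FOV, and outline toggling.
; Tick sphere-traces from the pawn to update the animal hint; J and H alert or move the nearest flock.
; Speed keys drive CheatManager Slomo, inversely scaling pawn speed to offset dilation.
; Sandbox mode broadcasts numbered actions, alongside trace-based helpers for spawning animals or food and killing animals.
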(event `Key|J`
  (params (Key :type "Key Structure"))
  (:`Pressed`
    (bind _outactors (`GameplayStatics.GetAllActorsOfClass` "/Game/BP/Flock/BP_FlockController.BP_FlockController_C"))
    (`/Game/BP/Flock/BP_FlockController.DangerPercievedNotify` (cast `/Game/BP/Flock/BP_FlockController` (`.ReturnValue` (`GameplayStatics.FindNearestActor` (`self.K2_GetActorLocation`) _outactors)) :!pure true) null)))

(event `Key|H`
  (params (Key :type "Key Structure"))
  (:`Pressed`
    (bind _outactors (`GameplayStatics.GetAllActorsOfClass` "/Game/BP/Flock/BP_FlockController.BP_FlockController_C"))
    (bind _location (`self.TraceFromCamera` (`|MakeArray` "ObjectTypeQuery1" :!type "EObjectTypeQuery Enum") 20000.0))
    (`/Game/BP/Flock/BP_FlockController.MoveFlock` (cast `/Game/BP/Flock/BP_FlockController` (`.ReturnValue` (`GameplayStatics.FindNearestActor` (`self.K2_GetActorLocation`) _outactors)) :!pure true) _location null)))

(event `InputAction|Pause`
  (params (Key :type "Key Structure"))
  ;[1 1 1] Pause
  (:`Pressed`
    (`GameplayStatics.SetGamePaused` true)
    (bind _returnvalue (`|CreateWidget` "/Game/Widgets/WBP_PauseMenu.WBP_PauseMenu_C"))
    (bind _output_get (set `self.PauseMenu` _returnvalue))
    (add `/Game/Widgets/WBP_PauseMenu.CloseRequest` _output_get (delegate `ClosePauseMenu`))
    (`UserWidget.AddToViewport` (`self.PauseMenu`) 0)
    (set `self.bShowMouseCursor` true)
    (`WidgetBlueprintLibrary.SetInputMode_UIOnlyEx` self (`self.PauseMenu`))
    ;[1 1 1] Settings
    (add `/Game/Widgets/WBP_PauseMenu.OpenSettingsRequest` (`self.PauseMenu`) (delegate `OpenSettings`))
    (`Widget.SetVisibility` (`self.CurrentHUDWidget`) "Collapsed")))

(event `ClosePauseMenu`
  ;[1 1 1] Pause
  (`GameplayStatics.SetGamePaused` false)
  (`Widget.RemoveFromParent` (`self.PauseMenu`))
  (`WidgetBlueprintLibrary.SetInputMode_GameOnly` self)
  (set `self.bShowMouseCursor` false)
  (set `self.PauseMenu` null)
  (`Widget.SetVisibility` (`self.CurrentHUDWidget`) "Visible"))

(event `OpenSettings`
  ;[1 1 1] Settings
  (bind _returnvalue (`|CreateWidget` "/Game/Widgets/WBP_Settings.WBP_Settings_C"))
  (add `/Game/Widgets/WBP_Settings.CloseRequest` _returnvalue (delegate `CloseRequest_Event_0`))
  (`UserWidget.AddToViewport` _returnvalue 0)
  (`Widget.SetVisibility` (`self.PauseMenu`) "Collapsed"))

(event `CloseRequest_Event_0`
  ;[1 1 1] Settings
  (`Widget.RemoveFromParent` (stale `OpenSettings` _returnvalue))
  (`Widget.SetVisibility` (`self.PauseMenu`) "Visible"))

(event `InputAction|SpeedMinus`
  (params (Key :type "Key Structure"))
  ;[1 1 1] GameSpeed
  (:`Pressed`
    (bind _output_get (set `self.TimeDilation` (`KismetMathLibrary.FClamp` (/ (`self.TimeDilation`) 2.0) 0.125 8.0)))
    (`CheatManager.Slomo` (`self.CheatManager`) _output_get)
    (`/Game/Widgets/WBP_MainHUD.UpdateTimeSpeedWidget` (`self.MainHUDWidget`) (`self.TimeDilation`) :!label _label)
    (set `FloatingPawnMovement.MaxSpeed` (/ (`self.PawnMovespeed`) (`self.TimeDilation`)) (cast `FloatingPawnMovement` (`Pawn.GetMovementComponent` (`GameplayStatics.GetPlayerPawn` 0)) :!pure true))))

(event `InputAction|SpeedPlus`
  (params (Key :type "Key Structure"))
  ;[1 1 1] GameSpeed
  (:`Pressed`
    (bind _output_get (set `self.TimeDilation` (`KismetMathLibrary.FClamp` (* (`self.TimeDilation`) 2.0) 0.125 8.0)))
    (`CheatManager.Slomo` (`self.CheatManager`) _output_get)
    (goto _label)))

(event `self.ReceiveBeginPlay`
  (bind _asbp_game_instance (cast `/Game/BP/BP_GameInstance` (`GameplayStatics.GetGameInstance`) :!pure true))
  ;[1 1 1] Widget Creation
  (bind _returnvalue (`|CreateWidget` "/Game/Widgets/WBP_FadeIn.WBP_FadeIn_C" null 9.0))
  (`UserWidget.AddToViewport` _returnvalue 9990)
  (bind _returnvalue_2 (`|CreateWidget` "/Game/Widgets/WBP_MainHUD.WBP_MainHUD_C"))
  (bind _output_get (set `self.MainHUDWidget` _returnvalue_2))
  (`UserWidget.AddToViewport` _output_get 0)
  (set `self.CurrentHUDWidget` (`self.MainHUDWidget`))
  (`WidgetBlueprintLibrary.SetInputMode_GameOnly` self)
  (bind _returnvalue_3 (`|CreateWidget` "/Game/Widgets/WBP_SandboxMenu.WBP_SandboxMenu_C"))
  (bind _output_get_2 (set `self.SandboxMenu` _returnvalue_3))
  (`UserWidget.AddToViewport` _output_get_2 0)
  (`Widget.SetVisibility` _output_get_2 "Collapsed")
  ;[1 1 1] Update stuff from settings
  (add `/Game/BP/BP_GameInstance.OnSensitivityUpdated` _asbp_game_instance (delegate `SensitivityUpdate`))
  (`self.SetSensitivity` (`/Game/BP/BP_GameInstance.GetSensitivity` _asbp_game_instance))
  (`KismetSystemLibrary.ExecuteConsoleCommand` (`KismetStringLibrary.Concat_StrStr` "fov " (`KismetStringLibrary.Conv_DoubleToString` (`/Game/BP/BP_GameInstance.FOV` _asbp_game_instance))) null))

(event `SensitivityUpdate`
  (params (NewValue :type "Float (double-precision)"))
  ;[1 1 1] Update stuff from settings
  (`self.SetSensitivity` NewValue))

(event `/Game/BP/BPI_Selectable.EntitySelected`
  (params (Entity :type "Actor Object Reference"))
  (`/Game/Widgets/WBP_AnimalHint.UpdateFromEntity` (`/Game/Widgets/WBP_MainHUD.WBP_AnimalHint` (`self.MainHUDWidget`)) Entity))

(event `self.ReceiveTick`
  (params (DeltaSeconds :type "Float (single-precision)"))
  (bind _returnvalue (`self.K2_GetPawn`))
  (bind _returnvalue_2 (`self.K2_GetActorLocation` _returnvalue))
  ;[1 1 1] Update UI hints about what we are looking at
  (bind _outhit (`KismetSystemLibrary.SphereTraceSingleForObjects` _returnvalue_2 (+ _returnvalue_2 (* (`self.GetActorForwardVector` _returnvalue) 10000.0)) 10.0 (`|MakeArray` "ObjectTypeQuery3" :!type "EObjectTypeQuery Enum") false (`|MakeArray` _returnvalue :!type "Actor Object Reference")))
  (`/Game/Widgets/WBP_AnimalHint.UpdateFromEntity` (`/Game/Widgets/WBP_MainHUD.WBP_AnimalHint` (`self.MainHUDWidget`)) (`.HitActor` (`GameplayStatics.BreakHitResult` _outhit))))

(event `InputAction|HideUI`
  (params (Key :type "Key Structure"))
  ;[1 1 1] UI/UX input
)

(event `InputAction|EnableOutline`
  (params (Key :type "Key Structure"))
  ;[1 1 1] UI/UX input
  (:`Pressed`
    (bind _outactors (`GameplayStatics.GetAllActorsWithInterface` "/Game/BP/BPI_Outline.BPI_Outline_C"))
    (for _array_element _outactors
      (message `/Game/BP/BPI_Outline.SetOutline` _array_element true)))
  (:`Released`
    (bind _outactors_2 (`GameplayStatics.GetAllActorsWithInterface` "/Game/BP/BPI_Outline.BPI_Outline_C"))
    (for _array_element_2 _outactors_2
      (message `/Game/BP/BPI_Outline.SetOutline` _array_element_2 false))))

(event `InputAction|ChangeUIMode`
  (params (Key :type "Key Structure"))
  (bind _sandboxmenu (`self.SandboxMenu`))
  (bind _mainhudwidget (`self.MainHUDWidget`))
  ;[1 1 1] UI/UX input
  (:`Pressed`
    (`Widget.SetVisibility` (`self.SandboxMenu`) "Collapsed")
    (`Widget.SetVisibility` (`self.MainHUDWidget`) "Collapsed")
    (set `self.SandboxMode` false)
    (bind _result (`/Engine/EditorBlueprintResources/StandardMacros.IncrementInt` (`self.UIMode`))
      (:`  `
        (if (== _result 3)
          (set `self.UIMode` 0))
        (switch `int` (`self.UIMode`)
          (:`0`
            (`Widget.SetVisibility` _mainhudwidget "Visible")
            (set `self.CurrentHUDWidget` _mainhudwidget))
          (:`1`
            (`Widget.SetVisibility` _sandboxmenu "Visible")
            (set `self.SandboxMode` true)
            (set `self.CurrentHUDWidget` _sandboxmenu)))))))

(event `InputAction|Action0`
  (params (Key :type "Key Structure"))
  (:`Pressed`
    (if (`self.SandboxMode`)
      (`self.OnActionOccured` 0))))

(event `InputAction|Action1`
  (params (Key :type "Key Structure"))
  (:`Pressed`
    (if (`self.SandboxMode`)
      (`self.OnActionOccured` 1))))

(event `InputAction|Action2`
  (params (Key :type "Key Structure"))
  (:`Pressed`
    (if (`self.SandboxMode`)
      (`self.OnActionOccured` 2))))

(event `InputAction|Action3`
  (params (Key :type "Key Structure"))
  (:`Pressed`
    (if (`self.SandboxMode`)
      (`self.OnActionOccured` 3))))

(event `InputAction|Action4`
  (params (Key :type "Key Structure"))
  (:`Pressed`
    (if (`self.SandboxMode`)
      (`self.OnActionOccured` 4))))

(event `InputAction|Action5`
  (params (Key :type "Key Structure"))
  (:`Pressed`
    (if (`self.SandboxMode`)
      (`self.OnActionOccured` 5))))

(fn `Kill`
  (bind (_location _hitactor) (`self.TraceFromCamera` (`|MakeArray` "ObjectTypeQuery3" :!type "EObjectTypeQuery Enum") 2000.0))
  (bind _asbp_animal_base (cast `/Game/BP/Animals/BP_AnimalBase` _hitactor))
  (`/Game/BP/Animals/BP_AnimalBase.Death` _asbp_animal_base))

(fn `MakeImmortal`)

(fn `SetSensitivity`
  (params (NewValue :type "Float (double-precision)"))
  (if (!= NewValue 0.0)
    (set `self.InputYawScale` (* 2.5 (`local.NewValue`)))
    (set `self.InputPitchScale` (* -2.5 (`local.NewValue`)))
    (set `self.InputRollScale` (* 1.0 (`local.NewValue`)))))

(fn `SpawnAnimal`
  (params (Class :type "/Game/BP/Animals/BP_AnimalBase Class Reference"))
  (bind _location (`self.TraceFromCamera` (`|MakeArray` "ObjectTypeQuery1" "ObjectTypeQuery2" :!type "EObjectTypeQuery Enum") 1000.0))
  (`|SpawnActorFromClass` (`local.Class`) (`KismetMathLibrary.MakeTransform` _location) "AdjustIfPossibleButAlwaysSpawn" "OverrideRootScale" null null))

(fn `SpawnFood`
  (params (Class :type "Actor Class Reference"))
  (bind _array (`|MakeArray` "ObjectTypeQuery1" :!type "EObjectTypeQuery Enum"))
  (bind _location (`self.TraceFromCamera` _array 2000.0))
  (`|SpawnActorFromClass` Class (`KismetMathLibrary.MakeTransform` (`/Game/BP/BP_FunctionLibrary.SnapToFloor` _location 2000.0 2000.0 _array)) "AdjustIfPossibleButAlwaysSpawn" "OverrideRootScale" null null))

(fn `TraceFromCamera`
  (params (ObjectTypes :type "Array of EObjectTypeQuery Enum (by ref)") (Distance :type "Float (double-precision)"))
  (returns (Location :type "Vector Structure") (HitActor :type "Actor Object Reference"))
  (bind _returnvalue (`self.K2_GetPawn`))
  (bind _returnvalue_2 (`self.K2_GetActorLocation` _returnvalue))
  (bind (_outhit _returnvalue_3) (`KismetSystemLibrary.LineTraceSingleForObjects` _returnvalue_2 (+ _returnvalue_2 (* (`self.GetActorForwardVector` _returnvalue) Distance)) ObjectTypes false (`|MakeArray` _returnvalue :!type "Actor Object Reference") "ForDuration"))
  (if _returnvalue_3
    (bind (_bblockinghit _binitialoverlap _time _distance _location _impactpoint _normal _impactnormal _physmat _hitactor _hitcomponent _hitbonename _hititem _elementindex _faceindex _tracestart _traceend) (`GameplayStatics.BreakHitResult` _outhit))
    (return _location _hitactor)
    (else
      (return _traceend null))))

(fn `UserConstructionScript`)