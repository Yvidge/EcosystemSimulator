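; BP_ExhaustionComponent is a component that tracks an exhaustion value which builds up over time.
; A looping timer started on BeginPlay drives periodic ticks in place of event Tick, each adding the default rate plus an adjustable accumulation.
; Getters, setters and adders expose both values, with exhaustion changes routed through SetExhaustion.
; SetExhaustion calls OnFullyExhausted whenever the unclamped value is at least 1.0.
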(event `self.ReceiveBeginPlay`
  (bind _returnvalue (`KismetSystemLibrary.K2_SetTimerDelegate` (`|CreateDelegate` :!event `ExhaustionTick`) (`self.Frequency`) true))
  (set `self.ExhaustionTickTimer` _returnvalue))

(fn `AddExhaustion`
  (params (Value :type "Float (double-precision)"))
  (`self.SetExhaustion` (+ Value (`self.GetExhaustion`))))

(fn `AddExhaustionAccumulation`
  (params (Value :type "Float (double-precision)"))
  (`self.SetExhaustionAccumulation` (+ (`self.GetExhaustionAccumulation`) Value)))

(fn `ExhaustionTick`
  (`self.AddExhaustion` (+ (`self.GetExhaustionAccumulation`) (`self.DefaultExhaustionAccumulation`))))

(fn `GetExhaustion`
  (returns (Exhaustion :type "Float (double-precision)"))
  (return (`self.Exhaustion`)))

(fn `GetExhaustionAccumulation`
  (returns (ExhaustionAccumulation :type "Float (double-precision)"))
  (return (`self.ExhaustionAccumulation`)))

(fn `SetExhaustion`
  (params (Exhaustion :type "Float (double-precision)"))
  (bind _output_get (set `self.Exhaustion` Exhaustion))
  (if (<= 1.0 _output_get)
    (`self.OnFullyExhausted`)))

(fn `SetExhaustionAccumulation`
  (params (ExhaustionAccumulation :type "Float (double-precision)"))
  (set `self.ExhaustionAccumulation` ExhaustionAccumulation))