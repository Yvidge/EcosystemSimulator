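; BP_StatisticsComponent is an actor component that registers its owning entity with the world statistics subsystem.
; On BeginPlay it reports a new entity using the owner's class and the Name from the owner's BP_UIDataComponent.
; On EndPlay it reports that an entity of that class is destroyed.
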(event `self.ReceiveBeginPlay`
  (bind _returnvalue (`self.GetOwner`))
  (`WorldStatisticsSubsystem.NewEntityCreated` (subsystem `WorldStatisticsSubsystem`) (`GameplayStatics.GetObjectClass` _returnvalue) (`KismetTextLibrary.Conv_TextToString` (`/Game/BP/Components/BP_UIDataComponent.Name` (`Actor.GetComponentByClass` _returnvalue "/Game/BP/Components/BP_UIDataComponent.BP_UIDataComponent_C")))))

(event `self.ReceiveEndPlay`
  (params (EndPlayReason :type "EEndPlayReason Enum" :default "Destroyed"))
  (`WorldStatisticsSubsystem.EntityDestroyed` (subsystem `WorldStatisticsSubsystem`) (`GameplayStatics.GetObjectClass` (`self.GetOwner`))))