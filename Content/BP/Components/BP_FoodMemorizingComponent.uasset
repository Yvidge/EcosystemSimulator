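; AI controller component that remembers locations where the controlled pawn has perceived edible food.
; A looping timer with randomized start polls perception, accumulating actors whose food component type matches the pawn's metabolism component.
; It stores the average location of all accumulated targets in FoodPlaces when the map is empty or any stored place lies beyond MaxRangeForPlace.
; GetFoodPlaces exposes the map, and optional debug spheres show new places.
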(event `self.ReceiveBeginPlay`
  (bind _updatefrequency (`self.UpdateFrequency`))
  (`KismetSystemLibrary.K2_SetTimerDelegate` (`|CreateDelegate` :!event `Update`) _updatefrequency true 0.0 _updatefrequency))

(fn `GetFoodPlaces`
  (returns (FoodPlaces :type "Map of Vector Structure to Float (double-precision)"))
  (return (`self.FoodPlaces`)))

(fn `IsUniqueLocation`
  (params (Loc :type "Vector Structure"))
  (returns (Unique :type Boolean))
  (bind _keys (`BlueprintMapLibrary.Map_Keys` (`self.FoodPlaces`)))
  (for _array_element _keys
    (if (> (`KismetMathLibrary.Vector_DistanceSquared` _array_element Loc) (`KismetMathLibrary.Square` (`self.MaxRangeForPlace`)))
      (return true)))
  (return (== (`KismetArrayLibrary.Array_Length` _keys) 0)))

(fn `Update`
  (locals (PerceptionComponent :type "AIPerceptionComponent Object Reference") (TargetFoodComponent :type "/Game/BP/Components/BP_FoodComponent Object Reference") (OwnerMetabolismComponent :type "/Game/BP/Components/BP_MetabolismComponent Object Reference") (Targets :type "Array of Actor Object Reference") (Pawn :type "Pawn Object Reference"))
  (bind _asaicontroller (cast `AIController` (`self.GetOwner`))
    (:`then`
      (set `local.PerceptionComponent` (`AIController.GetAIPerceptionComponent` _asaicontroller))
      (bind _output_get (set `local.Pawn` (`Controller.K2_GetPawn` _asaicontroller)))
      (`/Engine/EditorBlueprintResources/StandardMacros.IsValid` _output_get
        (:`Is Valid`
          (for _array_element (`AIPerceptionComponent.GetCurrentlyPerceivedActors` (`local.PerceptionComponent`) null)
            (set `local.TargetFoodComponent` (`Actor.GetComponentByClass` _array_element "/Game/BP/Components/BP_FoodComponent.BP_FoodComponent_C"))
            (set `local.OwnerMetabolismComponent` (`Actor.GetComponentByClass` (`local.Pawn`) "/Game/BP/Components/BP_MetabolismComponent.BP_MetabolismComponent_C"))
            (if (and (`KismetSystemLibrary.IsValid` (`local.TargetFoodComponent`)) (`KismetSystemLibrary.IsValid` (`local.OwnerMetabolismComponent`)))
              (if (`BlueprintGameplayTagLibrary.HasTag` (`/Game/BP/Components/BP_MetabolismComponent.PossibleFoodTypes` (`local.OwnerMetabolismComponent`)) (`/Game/BP/Components/BP_FoodComponent. FoodType` (`local.TargetFoodComponent`)) true)
                (`KismetArrayLibrary.Array_AddUnique` (`local.Targets`) _array_element))))
          (bind _returnvalue (`GameplayStatics.GetActorArrayAverageLocation` (`local.Targets`)))
          (if (`self.IsUniqueLocation` _returnvalue)
            (`BlueprintMapLibrary.Map_Add` (`self.FoodPlaces`) _returnvalue)
            (if (`self.ShowDebug`)
              (`KismetSystemLibrary.DrawDebugSphere` _returnvalue (/ (`self.MaxRangeForPlace`) 2.0) 12 (struct :`G` 1.0 :`B` 0.295923 :`A` 1.0) 10.0 10.0))))))
    (:`CastFailed`
      (`KismetSystemLibrary.PrintString` "Wrong place for component" true true (struct :`R` 1.0 :`B` 0.055809 :`A` 1.0)))))