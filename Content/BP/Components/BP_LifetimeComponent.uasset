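; BP_LifetimeComponent is a component that tracks its owner's age up to a maximum lifetime.
; A looping timer with a randomized start offset advances the age by tick frequency times an age multiplier, broadcasting each update and an ended event once the maximum is reached.
; An optional delayed step randomizes the starting age to a fraction of the maximum.
; Destruction broadcasts a died event, and getters expose current, maximum and normalized age.
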(event `self.ReceiveBeginPlay`
  (`KismetSystemLibrary.K2_SetTimerDelegate` (delegate `UpdateAge`) (`self.Frequency`) true 0.0 0.2)
  (`KismetSystemLibrary.Delay` 0.6)
  (if (`self.RandomizeInitialAge`)
    (set `self.CurrentAge` (`KismetMathLibrary.Conv_IntToDouble` (`KismetMathLibrary.FTrunc` (* (`KismetMathLibrary.RandomFloatInRange` 0.3 0.45) (`self.MaxAge`)))))))

(event `UpdateAge`
  (`|ExecutionSequence`
    (:`then_0`
      (bind _output_get (set `self.CurrentAge` (+ (`self.CurrentAge`) (* (`self.Frequency`) (`self.AgeMultiplier`)))))
      (`self.OnAgeUpdated` _output_get)
      (if (<= (`self.MaxAge`) _output_get)
        (`self.LifetimeEnded`)))))

(event `LifetimeEnded`
  (`self.OnLifetimeEnded`))

(event `self.ReceiveEndPlay`
  (params (EndPlayReason :type "EEndPlayReason Enum" :default "Destroyed"))
  (switch `EEndPlayReason` EndPlayReason
    (:`Destroyed`
      (`self.OnDied`))))

(fn `GetCurrentAge`
  (returns (CurrentAge :type "Float (double-precision)"))
  (return (`self.CurrentAge`)))

(fn `GetMaxAge`
  (returns (MaxAge :type "Float (double-precision)"))
  (return (`self.MaxAge`)))

(fn `GetNormalizedAge`
  (returns (NormalizedAge :type "Float (double-precision)"))
  (return (/ (`self.CurrentAge`) (`self.MaxAge`))))