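; Actor component that drives a creature's appearance by age and sex, active only when the owner has a BP_LifetimeComponent.
; At begin play it starts a looping timer, shares one dynamic material across owner-supplied meshes and applies the initial look.
; Curves sampled at normalized age optionally set the ColorModifier parameter and actor scale.
; Optional sexual dimorphism swaps skeletal meshes using the sex from BP_ReproductionComponent.
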(event `self.ReceiveBeginPlay`
  (bind _returnvalue (`Actor.GetComponentByClass` (`self.GetOwner`) "/Game/BP/Components/BP_LifetimeComponent.BP_LifetimeComponent_C"))
  (`/Engine/EditorBlueprintResources/StandardMacros.IsValid` _returnvalue
    (:`Is Valid`
      (bind _output_get (set `self.OwnerLifetimeComponenet` _returnvalue))
      (`self.AddTickPrerequisiteComponent` _output_get)
      (`KismetSystemLibrary.K2_SetTimerDelegate` (`|CreateDelegate` :!event `UpdateAppearance`) (`self.Frequency`) true 0.0 (`self.Initial Start Delay Variance`))
      (`self.InitilizeMaterial`)
      (`self.UpdateAppearance`)
      (`self.HandleSexualDemorphism`))))

(fn `HandleSexualDemorphism`
  (bind _returnvalue (`Actor.GetComponentByClass` (`self.GetOwner`) "/Game/BP/Components/BP_ReproductionComponent.BP_ReproductionComponent_C"))
  (if (`self.bSexualDemorphism`)
    (`/Engine/EditorBlueprintResources/StandardMacros.IsValid` _returnvalue
      (:`Is Valid`
        (bind _components (message `/Game/BP/BPI_AppearanceUpdate.GetAppearanceComponents` (`self.GetOwner`)))
        (for _array_element _components
          (bind _asskeletal_mesh_component (cast `SkeletalMeshComponent` _array_element))
          (`SkinnedMeshComponent.SetSkinnedAssetAndUpdate` _asskeletal_mesh_component (select `/Game/BP/SexEnum` (`/Game/BP/Components/BP_ReproductionComponent.Sex` _returnvalue) :`NewEnumerator0` (`self.FemaleMesh`) :`NewEnumerator1` (`self.MaleMesh`) :`NewEnumerator2` "/Engine/EditorMeshes/SkeletalMesh/DefaultSkeletalMesh.DefaultSkeletalMesh") true))))))

(fn `InitilizeMaterial`
  (bind _components (message `/Game/BP/BPI_AppearanceUpdate.GetComponentsToUpdateColor` (`self.GetOwner`)))
  (bind _returnvalue (`KismetMaterialLibrary.CreateDynamicMaterialInstance` (`PrimitiveComponent.GetMaterial` (cast `MeshComponent` (`|GetArrayItem` _components) :!pure true) 0)))
  (set `self.MaterialInstance` _returnvalue)
  (bind _components_2 (message `/Game/BP/BPI_AppearanceUpdate.GetComponentsToUpdateColor` (`self.GetOwner`)))
  (for _array_element _components_2
    (bind _asmesh_component (cast `MeshComponent` _array_element))
    (`PrimitiveComponent.SetMaterial` _asmesh_component 0 (`self.MaterialInstance`))))

(fn `SetColorTint`
  (params (Color :type "LinearColor Structure"))
  (`MaterialInstanceDynamic.SetVectorParameterValue` (`self.MaterialInstance`) "ColorModifier" Color))

(fn `SetMaterialColorParams`
  (`MaterialInstanceDynamic.SetVectorParameterValue` (`self.MaterialInstance`) "ColorModifier" (`CurveLinearColor.GetLinearColorValue` (`self.ColorCurve`) (`/Game/BP/Components/BP_LifetimeComponent.GetNormalizedAge` (`self.OwnerLifetimeComponenet`)))))

(fn `UpdateAppearance`
  (`|ExecutionSequence`
    (:`then_0`
      (if (`self.ChangeColor`)
        (`self.UpdateColor`)))
    (:`then_1`
      (if (`self.ChangeSize`)
        (`self.UpdateSize`)))))

(fn `UpdateColor`
  (`/Engine/EditorBlueprintResources/StandardMacros.IsValid` (`self.MaterialInstance`)
    (:`Is Valid`
      (`self.SetMaterialColorParams`))))

(fn `UpdateSize`
  (`Actor.SetActorScale3D` (`self.GetOwner`) (`KismetMathLibrary.Conv_DoubleToVector` (`CurveFloat.GetFloatValue` (`self.SizeCurve`) (`/Game/BP/Components/BP_LifetimeComponent.GetNormalizedAge` (`self.OwnerLifetimeComponenet`))))))