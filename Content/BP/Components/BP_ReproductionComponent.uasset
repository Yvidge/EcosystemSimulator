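; Actor component that lets its owner spawn copies of itself within a reproductive age window.
; It listens to the owner's BP_LifetimeComponent age updates and, when instant reproduction is enabled and age is in range, rolls a weighted chance.
; Success spawns the owner's class at a random nearby horizontal offset and yaw, avoiding collisions.
; A gate then blocks further attempts until the post-reproduction delay ends.
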(event `self.ReceiveBeginPlay`
  (bind _output_get (set `self.OwnerLifetimeComponent` (`Actor.GetComponentByClass` (`self.GetOwner`) "/Game/BP/Components/BP_LifetimeComponent.BP_LifetimeComponent_C")))
  (add `/Game/BP/Components/BP_LifetimeComponent.OnAgeUpdated` _output_get (delegate `OnOwnerAgeUpdated_Event`)))

(event `OnOwnerAgeUpdated_Event`
  (params (NewAge :type "Float (double-precision)"))
  (if (and (`self.IsReproductionInstant?`) (`self.CanReproduce?`))
    (`/Engine/EditorBlueprintResources/StandardMacros.Gate` false :!label _label
      (:`Exit`
        (bind _success_ (`self.Reproduce`))
        (if _success_
          (`|ExecutionSequence`
            (:`then_0`
              (goto _label :!via `Close`))
            (:`then_1`
              (`KismetSystemLibrary.Delay` (`self.DelayAfterReproduction`))
              (goto _label :!via `Open`))))))))

(fn `CanReproduce?`
  (returns (ReturnValue :type Boolean))
  (return (`KismetMathLibrary.InRange_FloatFloat` (`/Game/BP/Components/BP_LifetimeComponent.GetCurrentAge` (`self.OwnerLifetimeComponent`)) (`self.ReproductionStartAge`) (`self.ReproductionEndAge`))))

(fn `Reproduce`
  (returns (`Success?` :type Boolean))
  (bind _returnvalue (`self.GetOwner`))
  (if (`KismetMathLibrary.RandomBoolWithWeight` (`self.ChanceToReproduce`))
    (`|SpawnActorFromClass` (`GameplayStatics.GetObjectClass` _returnvalue) (`KismetMathLibrary.MakeTransform` (+ (`Actor.K2_GetActorLocation` _returnvalue) (`KismetMathLibrary.MakeVector` (`KismetMathLibrary.RandomFloatInRange` -500.0 500.0) (`KismetMathLibrary.RandomFloatInRange` -500.0 500.0))) (`KismetMathLibrary.MakeRotator` 0.0 0.0 (`KismetMathLibrary.RandomFloatInRange` 0.0 90.0))) "AdjustIfPossibleButDontSpawnIfColliding" "OverrideRootScale" null null)
    (return true)))