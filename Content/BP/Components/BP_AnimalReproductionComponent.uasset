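; Animal reproduction component that extends a parent reproduction component with mating, pregnancy and birth.
; StartBreeding also triggers the partner's component, and females or hermaphrodites become pregnant, gated by pregnancy, recovery and mating-state checks.
; Timers drive pregnancy and post-birth recovery, with a GAS Gameplay Effect applied for the pregnancy's duration.
; Birth uses parent spawning, fills newborns' metabolism calories to max, and pregnancy and birth post log messages.
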(event `self.ReceiveBeginPlay`
  (`parent.ReceiveBeginPlay`)
  (add `self.OnEntitiesSpawned` (delegate `SetChildrenHunger`)))

(event `SetChildrenHunger` :!signature `self.OnEntitiesSpawned`
  (params (SpawnedEntities :type "Array of Actor Object Reference (by ref)"))
  (for _array_element SpawnedEntities
    (bind _returnvalue (`Actor.GetComponentByClass` _array_element "/Game/BP/Components/BP_MetabolismComponent.BP_MetabolismComponent_C"))
    (`/Engine/EditorBlueprintResources/StandardMacros.IsValid` _returnvalue
      (:`Is Valid`
        (`/Game/BP/Components/BP_MetabolismComponent.SetCaloriesToMax` _returnvalue)))))

(fn `CanReproduce?`
  (returns (ReturnValue :type Boolean))
  (return (and (`parent.CanReproduce?`) (not (`self.Pregnant`)) (`self.RecoveredAfterPregnancy`) (not (`self.HavingSex`)))))

(fn `CopyFoodCacheToEntitiesSpawned`
  (params (SpawnedEntities :type "Array of Actor Object Reference (by ref)"))
  (for _ SpawnedEntities
    _))

(fn `EndPregnancy`
  (set `self.Pregnant` false)
  (`self.SpawnNewEntities`)
  (`KismetSystemLibrary.K2_SetTimerDelegate` (`|CreateDelegate` :!event `EndPregnancyRecover`) (`self.DelayAfterReproduction`))
  (`AbilitySystemComponent.RemoveActiveGameplayEffect` (`AbilitySystemBlueprintLibrary.GetAbilitySystemComponent` (`self.GetOwner`)) (`self.PregnancyEffectHandler`) -1))

(fn `EndPregnancyRecover`
  (set `self.RecoveredAfterPregnancy` true))

(fn `GetHavingSex`
  (returns (HavingSex :type Boolean))
  (return (`self.HavingSex`)))

(fn `IsPartnerSatisfying`
  (params (Partner :type "Actor Object Reference"))
  (returns (Answer :type Boolean))
  ;[1 1 1] Add some logic (age, health, etc)
  (return (and (`self.CanReproduce?` (`Actor.GetComponentByClass` Partner "BP_AnimalReproductionComponent_C")) (`self.CanReproduce?`))))

(fn `IsPregnant`
  (returns (Pregnant :type Boolean))
  (return (`self.Pregnant`)))

(fn `SetHavingSex`
  (params (Value :type Boolean))
  (set `self.HavingSex` Value))

(fn `SpawnNewEntities`
  (bind _returnvalue (`Actor.GetComponentByClass` (`self.GetOwner`) "/Game/BP/Components/BP_UIDataComponent.BP_UIDataComponent_C"))
  (`parent.SpawnNewEntities`)
  (`/Engine/EditorBlueprintResources/StandardMacros.IsValid` _returnvalue
    (:`Is Valid`
      (`/Game/BP/BP_FunctionLibrary.AddMessageToLog` (`|FormatText` "{Name} gave birth ({Num})" (`/Game/BP/Components/BP_UIDataComponent.Name` _returnvalue) (`self.NumBorn`)) (struct :`G` 0.45098 :`B` 0.101961 :`A` 1.0) 2.0))))

(fn `StartBreeding`
  (params (Partner :type "Actor Object Reference"))
  (`/Engine/EditorBlueprintResources/StandardMacros.IsValid` Partner
    (:`Is Valid`
      (`self.StartBreeding` (`Actor.GetComponentByClass` Partner "BP_AnimalReproductionComponent_C") null))
    (:`Is Not Valid`
      _))
  (switch `/Game/BP/SexEnum` (`self.Sex`)
    (:`NewEnumerator0`
      _)
    (:`NewEnumerator2`
      _))
  (`self.StartPregnancy`))

(fn `StartPregnancy`
  (bind _returnvalue (`Actor.GetComponentByClass` (`self.GetOwner`) "/Game/BP/Components/BP_UIDataComponent.BP_UIDataComponent_C"))
  (`KismetSystemLibrary.K2_SetTimerDelegate` (`|CreateDelegate` :!event `EndPregnancy`) (`self.PregnancyDuration`))
  (set `self.Pregnant` true)
  (set `self.RecoveredAfterPregnancy` false)
  (bind _returnvalue_2 (`AbilitySystemComponent.BP_ApplyGameplayEffectToSelf` :`self` (`AbilitySystemBlueprintLibrary.GetAbilitySystemComponent` (`self.GetOwner`)) :`GameplayEffectClass` "/Game/BP/GAS/GE_Pregnancy.GE_Pregnancy_C"))
  (set `self.PregnancyEffectHandler` _returnvalue_2)
  (`/Engine/EditorBlueprintResources/StandardMacros.IsValid` _returnvalue
    (:`Is Valid`
      (`/Game/BP/BP_FunctionLibrary.AddMessageToLog` (`|FormatText` "{Name} is pregnant" (`/Game/BP/Components/BP_UIDataComponent.Name` _returnvalue)) (struct :`G` 0.45098 :`B` 0.101961 :`A` 1.0) 2.0))))