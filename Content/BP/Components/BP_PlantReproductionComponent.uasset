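; Plant reproduction component that spawns new entities on a timer, building on a parent reproduction component.
; BeginPlay sets the first timer from ReproductionStartAge with random variance.
; The SpawnNewEntities override rolls a weighted chance before calling the parent's spawn, then always sets another timer using the post-reproduction delay.
; An older age-driven, gate-throttled path remains but is disabled, with its lifetime binding unconnected.
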(event `self.ReceiveBeginPlay`
  (`parent.ReceiveBeginPlay`)
  (`KismetSystemLibrary.K2_SetTimerDelegate` (`|CreateDelegate` :!event `SpawnNewEntities`) (`self.ReproductionStartAge`) false 0.0 (`self.ReproductionInitialDelayVarience`)))

(event `CustomEvent`
  (params (NewAge :type "Float (double-precision)"))
  (if (and false (`self.CanReproduce?`))
    (`/Engine/EditorBlueprintResources/StandardMacros.Gate` false :!label _label
      (:`Exit`
        (`self.SpawnNewEntities`)
        (if true
          (`|ExecutionSequence`
            (:`then_0`
              (goto _label :!via `Close`))
            (:`then_1`
              (`KismetSystemLibrary.Delay` (`self.DelayAfterReproduction`))
              (goto _label :!via `Open`))))))))

(event `self.ReceiveTick`
  (params (DeltaSeconds :type "Float (single-precision)")))

(fn `SpawnNewEntities`
  (if (`KismetMathLibrary.RandomBoolWithWeight` (`self.ChangeToReproduce`))
    (`parent.SpawnNewEntities`))
  (`KismetSystemLibrary.K2_SetTimerDelegate` (`|CreateDelegate` :!event `SpawnNewEntities`) (`self.DelayAfterReproduction`) false 0.0 (`self.ReproductionInitialDelayVarience`)))