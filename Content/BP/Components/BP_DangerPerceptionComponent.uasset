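; AI controller component that scores how dangerous each actor the controlled pawn currently sees is.
; CalculateDangerMap rebuilds an actor-to-danger map from sight perception on each call, and GetDangerMap returns it.
; Danger accumulates per actor: an optional flat score for meat eaters, plus scaled size for actors at or above a size gate.
; Actors of the pawn's own class add size danger only when explicitly enabled.
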(fn `CalculateDangerMap`
  (params (CheckDietType :type Boolean) (SizeGate :type "Float (double-precision)") (SizeDangerMultiplier :type "Float (double-precision)") (CalculateSizeDangerFromRelatives :type Boolean))
  (locals (`Controlled Pawn` :type "Pawn Object Reference") (Entity :type "Actor Object Reference"))
  (bind _returnvalue (`Actor.GetComponentByClass` (`local.Entity`) "/Game/BP/Components/BP_MetabolismComponent.BP_MetabolismComponent_C"))
  (bind _returnvalue_2 (`Actor.GetComponentByClass` (`local.Entity`) "/Game/BP/Components/BP_PhysicalParametersComponent.BP_PhysicalParametersComponent_C"))
  (bind _asaicontroller (cast `AIController` (`self.GetOwner`) :!pure true))
  (bind _size (`/Game/BP/Components/BP_PhysicalParametersComponent.GetSize` _returnvalue_2))
  (set `local.Controlled Pawn` (`Controller.K2_GetPawn` _asaicontroller))
  (`BlueprintMapLibrary.Map_Clear` (`self.PossibleDangers`))
  (for _array_element (`AIPerceptionComponent.GetCurrentlyPerceivedActors` (`AIController.GetAIPerceptionComponent` _asaicontroller) "/Script/AIModule.AISense_Sight")
    (set `local.Entity` _array_element)
    (`|ExecutionSequence`
      (:`then_0`
        (if (and (`local.CheckDietType`) (`KismetSystemLibrary.IsValid` _returnvalue))
          (if (`BlueprintGameplayTagLibrary.HasTag` (`/Game/BP/Components/BP_MetabolismComponent.PossibleFoodTypes` _returnvalue) (struct :`TagName` "Food.Meat") true)
            (`self.AddDanger` 10.0 (`local.Entity`)))))
      (:`then_1`
        (if (`KismetSystemLibrary.IsValid` _returnvalue_2)
          (if (<= (`local.SizeGate`) _size)
            (if (or (not (== (`GameplayStatics.GetObjectClass` (`local.Entity`)) (`GameplayStatics.GetObjectClass` (`local.Controlled Pawn`)))) (`local.CalculateSizeDangerFromRelatives`))
              (`self.AddDanger` (* _size (`local.SizeDangerMultiplier`)) (`local.Entity`))))))))
  (return))

(fn `GetDangerMap`
  (returns (PossibleDangers :type "Map of Actor Object Reference to Float (double-precision)"))
  (return (`self.PossibleDangers`)))