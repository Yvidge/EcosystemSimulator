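; Actor component that changes its owner's color and scale as the owner ages, using the owner's BP_LifetimeComponent.
; On BeginPlay it finds that component, sets a tick prerequisite on it, starts a looping timer and updates appearance.
; Optional color and size updates sample curves at normalized age.
; Color uses one lazily created dynamic material, applied to meshes the owner supplies through a message call.
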(event `self.ReceiveBeginPlay`
  (bind _returnvalue (`Actor.GetComponentByClass` (`self.GetOwner`) "/Game/BP/Components/BP_LifetimeComponent.BP_LifetimeComponent_C"))
  (`/Engine/EditorBlueprintResources/StandardMacros.IsValid` _returnvalue
    (:`Is Valid`
      (bind _output_get (set `self.OwnerLifetimeComponenet` _returnvalue))
      (`self.AddTickPrerequisiteComponent` _output_get)
      (`KismetSystemLibrary.K2_SetTimerDelegate` (`|CreateDelegate` :!event `UpdateAppearance`) (`self.Frequency`) true 0.0 (`self.Initial Start Delay Variance`))
      (`self.UpdateAppearance`))))

(fn `SetMaterialColorParams`
  (`MaterialInstanceDynamic.SetVectorParameterValue` (`self.MaterialInstance`) "Color" (`CurveLinearColor.GetLinearColorValue` (`self.ColorCurve`) (`/Game/BP/Components/BP_LifetimeComponent.GetNormalizedAge` (`self.OwnerLifetimeComponenet`)))))

(fn `UpdateAppearance`
  (`|ExecutionSequence`
    (:`then_0`
      (if (`self.ChangeColor`)
        (`self.UpdateColor`)))
    (:`then_1`
      (if (`self.ChangeSize`)
        (`self.UpdateSize`)))))

(fn `UpdateColor`
  (`/Engine/EditorBlueprintResources/StandardMacros.IsValid` (`self.MaterialInstance`)
    (:`Is Valid`
      _)
    (:`Is Not Valid`
      (bind _returnvalue (`KismetMaterialLibrary.CreateDynamicMaterialInstance` (`self.Material`)))
      (set `self.MaterialInstance` _returnvalue)
      (bind _components (message `/Game/BP/BPI_AppearanceUpdate.GetComponentsToUpdateColor` (`self.GetOwner`)))
      (for _array_element _components
        (bind _asmesh_component (cast `MeshComponent` _array_element))
        (`PrimitiveComponent.SetMaterial` _asmesh_component 0 (`self.MaterialInstance`)))))
  (`self.SetMaterialColorParams`))

(fn `UpdateSize`
  (`Actor.SetActorScale3D` (`self.GetOwner`) (`KismetMathLibrary.Conv_DoubleToVector` (`CurveFloat.GetFloatValue` (`self.SizeCurve`) (`/Game/BP/Components/BP_LifetimeComponent.GetNormalizedAge` (`self.OwnerLifetimeComponenet`))))))