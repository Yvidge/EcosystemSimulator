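; Food component that gives its owner a calorie store and a decay state.
; ConsumeCalories deducts up to the requested amount, reports how much was consumed, and fires CaloriesEnded when the store empties.
; A pausable looping timer drives decay from zero to one through Fresh, Carrion and Rot stages, firing OnDecayFinished at the end.
; CopyFromOuter copies calories, food type and decay settings from another component.
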(event `self.ReceiveBeginPlay`
  (if (== (`self.Calories`) 0.0)
    (set `self.Calories` (`self.DefaultCalories`))))

(fn `ConsumeCalories`
  (params (RequestedCalories :type "Float (double-precision)"))
  (returns (ConsumedCalories :type "Float (double-precision)") (IsRequestFullySatisfied :type Boolean))
  (locals (CaloriesConsumed :type "Float (double-precision)"))
  (if (<= RequestedCalories (`self.Calories`))
    (`self.SetCurrentCalories` (- (`self.Calories`) (`local.RequestedCalories`)))
    (if (`KismetMathLibrary.NearlyEqual_FloatFloat` (`self.Calories`))
      (`self.CaloriesEnded`))
    (return (`local.RequestedCalories`) true)
    (else
      (set `local.CaloriesConsumed` (`self.Calories`))
      (`self.SetCurrentCalories` 0.0)
      (`self.CaloriesEnded`)
      (return (`local.CaloriesConsumed`) false))))

(fn `Copy from Outer`
  (params (OuterComponent :type "/Game/BP/Components/BP_FoodComponent Object Reference"))
  (set `self.Decay` (`/Game/BP/Components/BP_FoodComponent.Decay` (`local.OuterComponent`)))
  (set `self.Calories` (`/Game/BP/Components/BP_FoodComponent.Calories` (`local.OuterComponent`)))
  (set `self.DefaultCalories` (`/Game/BP/Components/BP_FoodComponent.DefaultCalories` (`local.OuterComponent`)))
  (set `self. FoodType` (`/Game/BP/Components/BP_FoodComponent. FoodType` (`local.OuterComponent`)))
  (set `self.DecayTime` (`/Game/BP/Components/BP_FoodComponent.DecayTime` (`local.OuterComponent`)))
  (set `self.DecayUpdateFrequency` (`/Game/BP/Components/BP_FoodComponent.DecayUpdateFrequency` (`local.OuterComponent`))))

(fn `GetCurrentCalories`
  (returns (Calories :type "Float (double-precision)"))
  (return (`self.Calories`)))

(fn `GetDecay`
  (returns (Decay :type "Float (double-precision)"))
  (return (`self.Decay`)))

(fn `GetDecayStage`
  (returns (DecayStage :type "GameplayTag Structure"))
  (return (`self.DecayStage`)))

(fn `SetCurrentCalories`
  (params (Calories :type "Float (double-precision)"))
  (set `self.Calories` (`KismetMathLibrary.FClamp` Calories 0.0 10000.0)))

(fn `SetDecay`
  (params (Value :type "Float (double-precision)"))
  (bind _output_get (set `self.Decay` (`KismetMathLibrary.FClamp` Value)))
  (`self.UpdateDecayStage`)
  (if (== _output_get 1.0)
    (`self.OnDecayFinished`)))

(fn `StartDecay`
  (if (`KismetSystemLibrary.K2_TimerExistsHandle` (`self.DecayTimer`))
    (`KismetSystemLibrary.K2_UnPauseTimerHandle` (`self.DecayTimer`))
    (else
      (bind _returnvalue (`KismetSystemLibrary.K2_SetTimerDelegate` (`|CreateDelegate` :!event `UpdateDecay`) (`self.DecayUpdateFrequency`) true))
      (set `self.DecayTimer` _returnvalue))))

(fn `StopDecay`
  (if (`KismetSystemLibrary.K2_TimerExistsHandle` (`self.DecayTimer`))
    (`KismetSystemLibrary.K2_PauseTimerHandle` (`self.DecayTimer`))))

(fn `UpdateDecay`
  (`self.SetDecay` (+ (`self.GetDecay`) (/ (`self.DecayUpdateFrequency`) (`self.DecayTime`)))))

(fn `UpdateDecayStage`
  (if (<= (`self.GetDecay`) 0.3)
    (set `self.DecayStage` (struct :`TagName` "DecayStage.Fresh"))
    (elif (<= (`self.GetDecay`) 0.8)
      (set `self.DecayStage` (struct :`TagName` "DecayStage.Carrion"))
      (else
        (set `self.DecayStage` (struct :`TagName` "DecayStage.Rot"))))))