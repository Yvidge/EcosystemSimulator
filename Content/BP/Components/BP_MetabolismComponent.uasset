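; BP_MetabolismComponent is a component that tracks stored calories and hunger for its owner.
; A looping timer started on BeginPlay drives passive calorie burn, scaled by an adjustable multiplier, and empty storage starts half full.
; Every calorie change goes through one clamped setter, which maps the fill ratio through a curve to Hunger and fires OnCaloriesEnded at zero.
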(event `self.ReceiveBeginPlay`
  (`KismetSystemLibrary.K2_SetTimerDelegate` (`|CreateDelegate` :!event `CaloriesConsumptionTick`) (`self.PassiveCaloriesConsumptionFrequency`) true)
  (if (== (`self.CurrentCalories`) 0.0)
    (`self.SetCurrentCalories` (/ (`self.MaxCaloriesStored`) 2.0))))

(fn `AddCalories`
  (params (Num :type "Float (double-precision)"))
  (`self.SetCurrentCalories` (+ Num (`self.GetCurrentCalories`))))

(fn `CaloriesConsumptionTick`
  (`self.SetCurrentCalories` (- (`self.GetCurrentCalories`) (* (`self.PassiveCaloriesConsumption`) (`self.PassiveCaloriesConsumptionMultiplier`)))))

(fn `GetCaloriesNeededAmount`
  (returns (ReturnValue :type "Float (double-precision)"))
  (return (- (`self.MaxCaloriesStored`) (`self.CurrentCalories`))))

(fn `GetCurrentCalories`
  (returns (CurrentCalories :type "Float (double-precision)"))
  (return (`self.CurrentCalories`)))

(fn `GetHunger`
  (returns (Hunger :type "Float (double-precision)"))
  (return (`self.Hunger`)))

(fn `SetCurrentCalories`
  (params (NewValue :type "Float (double-precision)"))
  (bind _output_get (set `self.CurrentCalories` (`KismetMathLibrary.FClamp` NewValue 0.0 (`self.MaxCaloriesStored`))))
  (`self.SetHunger` (`CurveFloat.GetFloatValue` (`self.HungerCurve`) (/ _output_get (`self.MaxCaloriesStored`))))
  (if (`KismetMathLibrary.NearlyEqual_FloatFloat` (`self.GetCurrentCalories`))
    (`self.OnCaloriesEnded`)))

(fn `SetHunger`
  (params (Hunger :type "Float (double-precision)"))
  (set `self.Hunger` Hunger))

(fn `SetPassiveCaloriesConsumptionMultiplier`
  (params (PassiveCaloriesConsumptionMultiplier :type "Float (double-precision)"))
  (set `self.PassiveCaloriesConsumptionMultiplier` PassiveCaloriesConsumptionMultiplier))