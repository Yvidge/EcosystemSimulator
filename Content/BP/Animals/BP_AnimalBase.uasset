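; BP_AnimalBase is a base animal character that runs its primary behavior tree when an AI controller possesses it.
; Any damage, the end of its lifetime or calorie depletion kills it, spawning a BP_AnimalCorpse at its transform and destroying the actor.
; The corpse inherits the animal's food data through the food component's CopyFromOuter.
; Getter functions expose the mesh as the target for appearance, color and size updates.
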(event `self.ReceivePossessed`
  (params (NewController :type "Controller Object Reference"))
  (`AIController.RunBehaviorTree` (cast `AIController` NewController :!pure true) (`self.PrimaryBT`)))

(event `self.ReceiveAnyDamage`
  (params (Damage :type "Float (single-precision)") (DamageType :type "DamageType Object Reference") (InstigatedBy :type "Controller Object Reference") (DamageCauser :type "Actor Object Reference"))
  (bind _returnvalue (`|SpawnActorFromClass` "/Game/BP/Animals/BP_AnimalCorpse.BP_AnimalCorpse_C" (`self.GetTransform`) "AlwaysSpawn" "OverrideRootScale" null null :!label _label))
  (`/Game/BP/Components/BP_FoodComponent.Copy from Outer` (`/Game/BP/Animals/BP_AnimalCorpse.BP_FoodComponent` _returnvalue) (`self.BP_FoodComponent`))
  (`self.K2_DestroyActor`))

(event `self.BP_LifetimeComponent.OnLifetimeEnded`
  (goto _label))

(event `self.BP_MetabolismComponent.OnCaloriesEnded`
  (goto _label))

(fn `GetAppearanceComponents`
  (returns (Components :type "Array of SceneComponent Object Reference"))
  (return (`|MakeArray` (`self.Mesh`) :!type "SceneComponent Object Reference")))

(fn `GetComponentsToUpdateColor`
  (returns (Components :type "Array of SceneComponent Object Reference"))
  (return (`|MakeArray` (`self.Mesh`) :!type "SceneComponent Object Reference")))

(fn `GetComponentsToUpdateSize`
  (returns (Components :type "Array of SceneComponent Object Reference"))
  (return (`|MakeArray` (`self.Mesh`) :!type "SceneComponent Object Reference")))

(fn `UserConstructionScript`)