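; Zebra-specific flock component that sets species rules for forming and keeping animal flocks.
; When its owner matures as a male and is not the leader, it removes that animal from the flock.
; Flock creation requires both sexes plus the parent check.
; The initial-member filter flags the first male as leader pick but still returns every unique member, other males included.
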(event `self.ReceiveBeginPlay`
  (`parent.ReceiveBeginPlay`)
  (add `/Game/BP/Components/BP_AnimalReproductionComponent.OnBecameMature` (`Actor.GetComponentByClass` (`self.GetOwner`) "/Game/BP/Components/BP_AnimalReproductionComponent.BP_AnimalReproductionComponent_C") (delegate `HandleBecameMature`)))

(event `HandleBecameMature`
  (bind _flock (`self.GetFlock`))
  (if (and (`|EnumEquality` (`/Game/BP/Components/BP_ReproductionComponent.Sex` (`Actor.GetComponentByClass` (`self.GetOwner`) "/Game/BP/Components/BP_AnimalReproductionComponent.BP_AnimalReproductionComponent_C")) "NewEnumerator1") (not (`self.IsLeader`)))
    (`/Engine/EditorBlueprintResources/StandardMacros.IsValid` _flock
      (:`Is Valid`
        (`/Game/BP/Flock/BP_FlockController.RemoveFromFlock` _flock (`self.GetOwner`))))))

(fn `FilterInitialFlockMembers`
  (params (Members :type "Array of Actor Object Reference (by ref)"))
  (returns (FiltredMembers :type "Array of Actor Object Reference"))
  (locals (LeaderPicked :type Boolean) (LocalResult :type "Array of Actor Object Reference"))
  (for _array_element Members
    (if (and (`|EnumEquality` (`/Game/BP/Components/BP_ReproductionComponent.Sex` (`Actor.GetComponentByClass` _array_element "/Game/BP/Components/BP_ReproductionComponent.BP_ReproductionComponent_C")) "NewEnumerator1") (not (`local.LeaderPicked`)))
      (set `local.LeaderPicked` true)
      (`KismetArrayLibrary.Array_AddUnique` (`local.LocalResult`) _array_element)
      (else
        (`KismetArrayLibrary.Array_AddUnique` (`local.LocalResult`) _array_element))))
  (return (`local.LocalResult`)))

(fn `IsPossibleToCreateFlock?`
  (params (Members :type "Array of Actor Object Reference (by ref)"))
  (returns (Result :type Boolean))
  (locals (MaleInFlock :type Boolean) (FemaleInFlock :type Boolean))
  (for _array_element Members
    (if (`|EnumEquality` (`/Game/BP/Components/BP_ReproductionComponent.Sex` (`Actor.GetComponentByClass` _array_element "/Game/BP/Components/BP_ReproductionComponent.BP_ReproductionComponent_C")) "NewEnumerator1")
      (bind _output_get (set `local.MaleInFlock` true))
      (else
        (bind _output_get_2 (set `local.FemaleInFlock` true))))
    (bind _returnvalue (and _output_get _output_get_2))
    (if _returnvalue
      (return (and (`parent.IsPossibleToCreateFlock?` (`local.Members`)) (`local.MaleInFlock`) _returnvalue))))
  (return false))