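; Flock controller that groups animals under a leader and coordinates their movement, foraging and escape from danger.
; It tracks members through BP_FlockComponent and periodically updates leader-weighted bounds with debug circles.
; Hunger and danger notifications pick destinations from cached food or EQS queries, then give members offset targets and switch their behavior trees.
; Destruction possesses a temporary pawn and detaches it, apparently an engine workaround.
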(event `self.ReceiveBeginPlay`
  (`self.Initialize`)
  (`KismetSystemLibrary.K2_SetTimerDelegate` (`|CreateDelegate` :!event `UpdateFlockBounds`) (`self.BoundsUpdateFrequency`) true)
  (add `self.OnNewMemberJoined` (delegate `OnNewMemberJoined_Event`)))

(event `OnNewMemberJoined_Event` :!signature `self.OnNewMemberJoined`
  (params (NewMember :type "Actor Object Reference"))
  (if (not (`self.FlockHasLeader`))
    (if (`self.CanBeLeader` NewMember)
      (`self.SetLeader` NewMember))))

(event `Destroy`
  ;[1 1 1] Thanks UE
  (bind _returnvalue (`|SpawnActorFromClass` "/Game/BP/Flock/BP_FlockTMPPawn.BP_FlockTMPPawn_C" (`KismetMathLibrary.MakeTransform` (0.0 0.0 0.0)) "AlwaysSpawn" "OverrideRootScale" null null))
  (`KismetSystemLibrary.Delay` 0.2)
  (`self.Possess` _returnvalue)
  (`Pawn.DetachFromControllerPendingDestroy` _returnvalue))

(fn `AddToFlock`
  (params (TargetToAdd :type "Actor Object Reference"))
  (returns (`Return value` :type Boolean))
  (bind _targettoadd (`local.TargetToAdd`))
  (if (`self.CanBeMember` TargetToAdd)
    (`KismetArrayLibrary.Array_AddUnique` (`self.Members`) _targettoadd)
    (`self.OnNewMemberJoined` _targettoadd)
    (`/Game/BP/Flock/BP_FlockComponent.SetFlock` (`self.GetComponentByClass` _targettoadd "/Game/BP/Flock/BP_FlockComponent.BP_FlockComponent_C") self)
    (if (not (`self.FlockMoving`))
      (return true)
      (else
        (`self.HandleAddWhileMoving` (`local.TargetToAdd`))
        (return true)))
    (else
      (return false))))

(fn `CanBeLeader`
  (params (Target :type "Actor Object Reference"))
  (returns (`Return value` :type Boolean))
  (return (`KismetSystemLibrary.IsValid` Target)))

(fn `CanBeMember`
  (params (Target :type "Actor Object Reference"))
  (returns (Result :type Boolean))
  (return (`KismetSystemLibrary.IsValid` Target)))

(fn `ChooseLeader`
  (returns (Successfully :type Boolean))
  (locals (LocalCandidates :type "Array of Actor Object Reference"))
  (for _array_element (`self.Members`)
    (if (`self.CanBeLeader` _array_element)
      (`KismetArrayLibrary.Array_AddUnique` (`local.LocalCandidates`) _array_element)))
  (bind _result (`self.PickBestLeader` (`local.LocalCandidates`)))
  (`/Engine/EditorBlueprintResources/StandardMacros.IsValid` _result
    (:`Is Valid`
      (`self.SetLeader` _result)
      (return true))
    (:`Is Not Valid`
      (return false))))

(fn `DangerPercievedNotify`
  (params (Member :type "Actor Object Reference"))
  (`KismetSystemLibrary.PrintString` (`KismetSystemLibrary.GetDisplayName` Member))
  (`KismetSystemLibrary.K2_SetTimerDelegate` (`|CreateDelegate` :!event `UpdateEscapeLocation`) (`self.EscapeLocationUpdateFrequency`) true)
  (bind _returnvalue (`EnvQueryManager.RunEQSQuery` "/Game/AI/EQS/EQS_FlockEscapeLocation.EQS_FlockEscapeLocation" (`|GetArrayItem` (`self.Members`)) "RandomBest5Pct"))
  (add `EnvQueryInstanceBlueprintWrapper.OnQueryFinishedEvent` _returnvalue (`|CreateDelegate` :!event `EscapeLocationEQSFinished`)))

(fn `DestroyFlock`
  (for _array_element (`self.Members`)
    (`/Game/BP/Flock/BP_FlockComponent.HandleFlockLeaving` (`self.GetComponentByClass` _array_element "/Game/BP/Flock/BP_FlockComponent.BP_FlockComponent_C")))
  (`self.Destroy`))

(fn `EscapeLocationEQSFinished`
  (params (QueryInstance :type "EnvQueryInstanceBlueprintWrapper Object Reference") (QueryStatus :type "EEnvQueryStatus Enum" :default "Processing"))
  (bind (_resultlocations _returnvalue) (`EnvQueryInstanceBlueprintWrapper.GetQueryResultsAsLocations` QueryInstance))
  (if _returnvalue
    (`self.MoveFlock` (`|GetArrayItem` _resultlocations) "/Game/AI/BehaviorTrees/BT_FlockMemberRunFromDanger.BT_FlockMemberRunFromDanger")
    (if (not (`KismetSystemLibrary.K2_TimerExistsHandle` (`self.DangerObservationTimer`)))
      (bind _returnvalue_2 (`KismetSystemLibrary.K2_SetTimerDelegate` (`|CreateDelegate` :!event `ObserveMembersOutOfDanger`) 0.6 true))
      (set `self.DangerObservationTimer` _returnvalue_2))))

(fn `FlockHasLeader`
  (returns (`Return Value` :type Boolean))
  (return (`KismetSystemLibrary.IsValid` (`self.Leader`))))

(fn `FoodFindingEQSFinished`
  (params (QueryInstance :type "EnvQueryInstanceBlueprintWrapper Object Reference") (QueryStatus :type "EEnvQueryStatus Enum" :default "Processing"))
  (bind (_resultlocations _returnvalue) (`EnvQueryInstanceBlueprintWrapper.GetQueryResultsAsLocations` QueryInstance))
  (if _returnvalue
    (`self.MoveFlock` (`|GetArrayItem` _resultlocations) "/Game/AI/BehaviorTrees/BT_FlockMemberMoveFindFood.BT_FlockMemberMoveFindFood")))

(fn `FoodFoundNotify`
  (params (FoodActor :type "Actor Object Reference"))
  (`self.MoveFlock` (`self.K2_GetActorLocation` FoodActor)))

(fn `GenerateTargetMoveLocations`
  (params (TargetLoc :type "Vector Structure" :default (0.0 0.0 0.0)))
  (locals (Map :type "Map of Actor Object Reference to Vector Structure"))
  (bind _bounds_origin (`KismetMathLibrary.BreakBoxSphereBounds` (`self.Bounds`)))
  (for _array_element (`self.Members`)
    (`BlueprintMapLibrary.Map_Add` (`local.Map`) _array_element (+ (- (`self.K2_GetActorLocation` _array_element) _bounds_origin) (`local.TargetLoc`))))
  (set `self.TargetLocations` (`local.Map`)))

(fn `GetAllKnownDangers`
  (returns (`Return Value` :type "Array of Actor Object Reference"))
  (locals (LocalResults :type "Array of Actor Object Reference"))
  (for _array_element (`self.Members`)
    (bind _returnvalue (`AIBlueprintHelperLibrary.GetAIController` _array_element))
    (`/Engine/EditorBlueprintResources/StandardMacros.IsValid` _returnvalue
      (:`Is Valid`
        (bind _keys (`BlueprintMapLibrary.Map_Keys` (`/Game/BP/Components/BP_DangerPerceptionComponent.GetDangerMap` (`self.GetComponentByClass` _returnvalue "/Game/BP/Components/BP_DangerPerceptionComponent.BP_DangerPerceptionComponent_C"))))
        (for _array_element_2 _keys
          (`KismetArrayLibrary.Array_AddUnique` (`local.LocalResults`) _array_element_2)))))
  (return (`local.LocalResults`)))

(fn `GetFlockBounds`
  (returns (Bounds :type "BoxSphereBounds Structure"))
  (return (`self.Bounds`)))

(fn `GetLeader`
  (returns (Leader :type "Actor Object Reference"))
  (return (`self.Leader`)))

(fn `GetMembers`
  (returns (Members :type "Array of Actor Object Reference"))
  (return (`self.Members`)))

(fn `GetMoveLocation`
  (params (Actor :type "Actor Object Reference"))
  (returns (CalculatedLocation :type "Vector Structure"))
  (bind (_value _returnvalue) (`BlueprintMapLibrary.Map_Find` (`self.TargetLocations`) Actor))
  (if _returnvalue
    (return _value)
    (else
      (return (0.0 0.0 0.0)))))

(fn `GetSexRequestFlockOverride`
  (params (SourceMember :type "Actor Object Reference") (TargetMember :type "Actor Object Reference"))
  (returns (`Return Value` :type Boolean))
  (return (== TargetMember (`self.Leader`))))

(fn `HandleAddWhileMoving`
  (params (TargetMember :type "Actor Object Reference"))
  (bind _returnvalue (`AIBlueprintHelperLibrary.GetAIController` (`local.TargetMember`)))
  (`BlueprintMapLibrary.Map_Add` (`self.TargetLocations`) (`local.TargetMember`) (`self.LastTargetLocation`))
  (`/Engine/EditorBlueprintResources/StandardMacros.IsValid` _returnvalue
    (:`Is Valid`
      (`self.RunBehaviorTree` _returnvalue (`self.FlockMoveBT`)))))

(fn `HungerNotify`
  (if (not (`self.FlockMoving`))
    (for _array_element (`self.Members`)
      (bind _returnvalue (`self.GetComponentByClass` (`AIBlueprintHelperLibrary.GetAIController` _array_element) "/Game/BP/Components/BP_MemoryCacheComponent.BP_MemoryCacheComponent_C"))
      (`/Engine/EditorBlueprintResources/StandardMacros.IsValid` _returnvalue
        (:`Is Valid`
          (for _array_element_2 (`/Game/BP/Components/BP_MemoryCacheComponent.GetFoodCache` _returnvalue)
            (`/Engine/EditorBlueprintResources/StandardMacros.IsValid` _array_element_2
              (:`Is Valid`
                (`self.MoveFlock` (`self.K2_GetActorLocation` _array_element_2) "/Game/AI/BehaviorTrees/BT_FlockMemberMoveTo.BT_FlockMemberMoveTo")
                (return)))))))
    (bind _returnvalue_2 (`EnvQueryManager.RunEQSQuery` (`self.FoodFindingQueryTemplate`) (`|GetArrayItem` (`self.Members`)) "RandomBest25Pct"))
    (add `EnvQueryInstanceBlueprintWrapper.OnQueryFinishedEvent` _returnvalue_2 (`|CreateDelegate` :!event `FoodFindingEQSFinished`))
    (set `self.FlockMoving` true)))

(fn `Initialize`
  (`self.InitializeFlockColor`)
  (for _array_element (`self.Members`)
    (`/Game/BP/Flock/BP_FlockComponent.SetFlock` (`self.GetComponentByClass` _array_element "/Game/BP/Flock/BP_FlockComponent.BP_FlockComponent_C") self))
  (bind _successfully (`self.ChooseLeader`))
  (if (not _successfully)
    (`KismetSystemLibrary.PrintString` "No leader found " true true (`self.FlockColor`))))

(fn `InitializeFlockColor`
  (set `self.FlockColor` (make `LinearColor` (`KismetMathLibrary.RandomFloatInRange` 0.0 1.0) (`KismetMathLibrary.RandomFloatInRange` 0.0 1.0) (`KismetMathLibrary.RandomFloatInRange` 0.0 1.0) 1.0))
  (return))

(fn `IsAnyMemberFeelDanger`
  (returns (`Return Value` :type Boolean))
  (locals (DangerNearby :type Boolean))
  (set `local.DangerNearby` false)
  (for _array_element (`self.Members`)
    (bind _returnvalue (`AIBlueprintHelperLibrary.GetBlackboard` _array_element))
    (`/Engine/EditorBlueprintResources/StandardMacros.IsValid` _returnvalue
      (:`Is Valid`
        (set `local.DangerNearby` (or (`local.DangerNearby`) (not (== (`BlackboardComponent.GetValueAsFloat` _returnvalue "DangerLevel") 0.0)))))))
  (return (`local.DangerNearby`)))

(fn `Merge`)

(fn `MoveFinishedNotify`
  (set `self.FlockMoving` false)
  (for _array_element (`self.Members`)
    (bind _returnvalue (`AIBlueprintHelperLibrary.GetAIController` _array_element))
    (`/Engine/EditorBlueprintResources/StandardMacros.IsValid` _returnvalue
      (:`Is Valid`
        (`self.RunBehaviorTree` _returnvalue "/Game/AI/BehaviorTrees/BT_AnimalBase.BT_AnimalBase")))))

(fn `MoveFlock`
  (params (TargetLoc :type "Vector Structure") (BTOverride :type "BehaviorTree Object Reference"))
  (`self.GenerateTargetMoveLocations` TargetLoc)
  (set `self.FlockMoving` true)
  (set `self.LastTargetLocation` (`local.TargetLoc`))
  (for _array_element (`self.Members`)
    (bind _returnvalue (`AIBlueprintHelperLibrary.GetAIController` _array_element))
    (`/Engine/EditorBlueprintResources/StandardMacros.IsValid` _returnvalue
      (:`Is Valid`
        (`self.RunBehaviorTree` _returnvalue (select `bool` (`KismetSystemLibrary.IsValid` (`local.BTOverride`)) :`false` (`self.FlockMoveBT`) :`true` (`local.BTOverride`)))))))

(fn `ObserveMembersOutOfDanger`
  (locals (DangerNearby :type Boolean))
  (if (not (`self.IsAnyMemberFeelDanger`))
    (`self.SetFlockBT` "/Game/AI/BehaviorTrees/BT_AnimalBase.BT_AnimalBase")
    (`KismetSystemLibrary.K2_ClearAndInvalidateTimerHandle` (`self.DangerObservationTimer`))))

(fn `OnNewEscapeLocationsGenerated`
  (params (QueryInstance :type "EnvQueryInstanceBlueprintWrapper Object Reference") (QueryStatus :type "EEnvQueryStatus Enum" :default "Processing"))
  (bind (_resultlocations _returnvalue) (`EnvQueryInstanceBlueprintWrapper.GetQueryResultsAsLocations` QueryInstance))
  (if _returnvalue
    (`self.GenerateTargetMoveLocations` (`|GetArrayItem` _resultlocations))
    (for _array_element (`self.Members`)
      (bind _returnvalue_2 (`AIBlueprintHelperLibrary.GetBlackboard` _array_element))
      (`/Engine/EditorBlueprintResources/StandardMacros.IsValid` _returnvalue_2
        (:`Is Valid`
          (`BlackboardComponent.SetValueAsVector` _returnvalue_2 "TargetLocation" (`self.GetMoveLocation` _array_element)))))))

(fn `PickBestLeader`
  (params (Candidates :type "Array of Actor Object Reference"))
  (returns (Result :type "Actor Object Reference"))
  (return (`|GetArrayItem` Candidates)))

(fn `RemoveFromFlock`
  (params (TargetToRemove :type "Actor Object Reference"))
  (returns (ReturnValue :type Boolean))
  (bind _returnvalue (`KismetArrayLibrary.Array_RemoveItem` (`self.Members`) (`local.TargetToRemove`)))
  (if _returnvalue
    (`/Game/BP/Flock/BP_FlockComponent.HandleFlockLeaving` (`self.GetComponentByClass` (`local.TargetToRemove`) "/Game/BP/Flock/BP_FlockComponent.BP_FlockComponent_C"))
    (`self.OnMemberDisjoined` (`local.TargetToRemove`))
    (if (>= (`KismetArrayLibrary.Array_Length` (`self.Members`)) 2)
      (return true)
      (else
        (`self.DestroyFlock`)
        (return true)))
    (else
      (return false))))

(fn `SetFlockBT`
  (params (BT :type "BehaviorTree Object Reference"))
  (for _array_element (`self.Members`)
    (bind _returnvalue (`AIBlueprintHelperLibrary.GetAIController` _array_element))
    (`/Engine/EditorBlueprintResources/StandardMacros.IsValid` _returnvalue
      (:`Is Valid`
        (`self.RunBehaviorTree` _returnvalue (`local.BT`))))))

(fn `SetLeader`
  (params (Leader :type "Actor Object Reference"))
  (locals (OldLeader :type "Actor Object Reference"))
  (bind _leader (`self.GetLeader`))
  (if (!= Leader (`self.GetLeader`))
    (bind _output_get (set `local.OldLeader` _leader))
    (`/Engine/EditorBlueprintResources/StandardMacros.IsValid` _output_get
      (:`Is Valid`
        (`/Game/BP/Flock/BP_FlockComponent.SetLeader` (`self.GetComponentByClass` _leader "/Game/BP/Flock/BP_FlockComponent.BP_FlockComponent_C") false))
      (:`Is Not Valid`
        _))
    (bind _output_get_2 (set `self.Leader` Leader))
    (`/Game/BP/Flock/BP_FlockComponent.SetLeader` (`self.GetComponentByClass` _output_get_2 "/Game/BP/Flock/BP_FlockComponent.BP_FlockComponent_C") true)
    (`self.OnLeaderChanged` (`self.Leader`) (`local.OldLeader`))))

(fn `UpdateEscapeLocation`
  (bind _returnvalue (`EnvQueryManager.RunEQSQuery` "/Game/AI/EQS/EQS_FlockEscapeLocation.EQS_FlockEscapeLocation" (`|GetArrayItem` (`self.Members`)) "RandomBest5Pct"))
  (add `EnvQueryInstanceBlueprintWrapper.OnQueryFinishedEvent` _returnvalue (`|CreateDelegate` :!event `OnNewEscapeLocationsGenerated`)))

(fn `UpdateFlockBounds`
  (bind _returnvalue (`GameplayStatics.GetActorArrayAverageLocation` (`self.Members`)))
  (bind _structout (setmembers `BoxSphereBounds` :`StructRef` (`self.Bounds`) :`Origin` (`KismetMathLibrary.SelectVector` (`KismetMathLibrary.VLerp` _returnvalue (`self.K2_GetActorLocation` (`self.GetLeader`)) 0.3) _returnvalue (`self.FlockHasLeader`))))
  (bind (_origin _boxextent _sphereradius) (`KismetMathLibrary.BreakBoxSphereBounds` _structout))
  (`KismetSystemLibrary.DrawDebugCircle` _origin _sphereradius 24 (`self.FlockColor`) (`self.BoundsUpdateFrequency`) 5.0 (0.0 1.0 0.0) (1.0 0.0 0.0))
  (if (`self.FlockHasLeader`)
    (`KismetSystemLibrary.DrawDebugCircle` (`self.K2_GetActorLocation` (`self.Leader`)) 50.0 12 (struct :`R` 1.0 :`G` 1.0 :`B` 1.0 :`A` 1.0) (`self.BoundsUpdateFrequency`) 3.0 (0.0 1.0 0.0) (1.0 0.0 0.0))))

(fn `UserConstructionScript`)