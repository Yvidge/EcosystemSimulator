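; Zebra flock controller that specializes the parent's rules for which animals can lead or join a flock.
; CanBeLeader accepts only animals of one specific sex, read from their reproduction component.
; CanBeMember admits that same sex only if the animal is a child or the flock has no leader.
; Both overrides also require the parent check to pass, which is the only membership test for other animals.
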(fn `CanBeLeader`
  (params (Target :type "Actor Object Reference"))
  (returns (`Return value` :type Boolean))
  (return (and (`|EnumEquality` (`/Game/BP/Components/BP_ReproductionComponent.Sex` (`self.GetComponentByClass` Target "/Game/BP/Components/BP_AnimalReproductionComponent.BP_AnimalReproductionComponent_C")) "NewEnumerator1") (`parent.CanBeLeader` (`local.Target`)))))

(fn `CanBeMember`
  (params (Target :type "Actor Object Reference"))
  (returns (Result :type Boolean))
  (if (`|EnumEquality` (`/Game/BP/Components/BP_ReproductionComponent.Sex` (`self.GetComponentByClass` (`local.Target`) "/Game/BP/Components/BP_ReproductionComponent.BP_ReproductionComponent_C")) "NewEnumerator1")
    (return (and (or (`/Game/BP/Components/BP_AnimalReproductionComponent.IsChild` (`self.GetComponentByClass` (`local.Target`) "/Game/BP/Components/BP_AnimalReproductionComponent.BP_AnimalReproductionComponent_C")) (not (`self.FlockHasLeader`))) (`parent.CanBeMember` (`local.Target`))))
    (else
      (return (`parent.CanBeMember` (`local.Target`))))))

(fn `UserConstructionScript`
  (`parent.UserConstructionScript`))