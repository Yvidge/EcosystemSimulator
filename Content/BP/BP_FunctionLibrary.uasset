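; Blueprint function library with two helpers: a sex compatibility check and a nearest-location search.
; IsSexPossible returns true when the first sex is one specific enum value, otherwise only when the two sexes differ.
; FindNearestLocation loops over candidate vectors and returns the closest to a source with its squared distance, or a zero vector and -1 for an empty array.
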(fn `FindNearestLocation`
  (params (Source :type "Vector Structure") (Locations :type "Array of Vector Structure"))
  (returns (Location :type "Vector Structure") (Distance :type "Float (double-precision)"))
  (locals (MinDistance :type "Float (double-precision)" :default 9999999.0) (ResultLocation :type "Vector Structure"))
  (if (!= (`KismetArrayLibrary.Array_Length` Locations) 0)
    (for _array_element (`local.Locations`)
      (bind _returnvalue (`KismetMathLibrary.Vector_DistanceSquared` _array_element (`local.Source`)))
      (if (< _returnvalue (`local.MinDistance`))
        (set `local.MinDistance` _returnvalue)
        (set `local.ResultLocation` _array_element)))
    (return (`local.ResultLocation`) (`local.MinDistance`))
    (else
      (return (0.0 0.0 0.0) -1.0))))

(fn `IsSexPossible`
  (params (Sex1 :type "/Game/BP/Enums/SexEnum Enum" :default "NewEnumerator0") (Sex2 :type "/Game/BP/Enums/SexEnum Enum" :default "NewEnumerator0"))
  (returns (Possible :type Boolean))
  (if (`|EnumEquality` Sex1 "NewEnumerator2")
    (return true)
    (else
      (return (`|EnumInequality` Sex1 Sex2)))))